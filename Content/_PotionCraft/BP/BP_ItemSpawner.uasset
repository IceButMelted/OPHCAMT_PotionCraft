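; BP_ItemSpawner is a respawning item spawner that replaces its item of class ClassFilter whenever that item leaves its check box.
; BeginPlay spawns the first item just above the root if none is valid and tracks it as CurrentFocusObject.
; When that actor ends overlap with BoxCheckItemIn, SpawnItem creates a replacement.
; Begin overlap only sets a flag and prints debug text, and older count-based spawn logic is disconnected.
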(event OnComponentBeginOverlap(BoxCheckitemIn)
  (params (OverlappedComponent :type Primitive%20Component%20Object%20Reference) (OtherActor :type Actor%20Object%20Reference) (OtherComp :type Primitive%20Component%20Object%20Reference) (OtherBodyIndex :type Integer) (bFromSweep :type Boolean) (SweepResult :type Hit%20Result%20Structure%20%28by%20ref%29))
  ;[0.4724 1 0.3075] Comment
  (if (== (Utilities|GetClass OtherActor) (Variables|Default|GetClass%20Filter))
    (Variables|Default|SetIsitemToSpawnInSide? true)
    (Development|PrintString "object to spawn is overlap" true true "(R=0.395378,G=0.000000,B=1.000000,A=1.000000)")
    (else
      (Variables|Default|SetIsitemToSpawnInSide? false)
      (Development|PrintString "object to spawn isn't overlap" true true "(R=1.000000,G=0.000000,B=0.218558,A=1.000000)"))))

(event OnComponentEndOverlap(BoxCheckitemIn)
  (params (OverlappedComponent :type Primitive%20Component%20Object%20Reference) (OtherActor :type Actor%20Object%20Reference) (OtherComp :type Primitive%20Component%20Object%20Reference) (OtherBodyIndex :type Integer))
  ;[0.1912 0.4072 0.1248] Comment
  (if (== OtherActor (Variables|Default|GetCurrentFocusObject))
    (Variables|Default|GetCurrentFocusObject
      (:then
        (Variables|Default|SetCurrentFocusObject 0)
        (CallFunction|SpawnItem))
      (:else))))

(event Custom|SpawnItem
  (bind _defaultsceneroot (Variables|Default|GetDefaultSceneRoot))
  (bind _returnvalue (Transformation|GetWorldLocation _defaultsceneroot))
  (bind (_x _y _z) (Math|Vector|BreakVector _returnvalue))
  ;[0.1912 0.4072 0.1248] Comment
  (bind _returnvalue_2 (Game|SpawnActorfromClass (Variables|Default|GetClass%20Filter) (Math|Transform|MakeTransform (Math|Vector|MakeVector _x _y (+ _z 1e+01)) "0, 0, 0" "1.000000,1.000000,1.000000") "Undefined" "MultiplyWithRoot" 0 0))
  (Variables|Default|SetCurrentFocusObject _returnvalue_2))

(event EventBeginPlay
  (bind _defaultsceneroot (Variables|Default|GetDefaultSceneRoot))
  (bind _returnvalue (Transformation|GetWorldLocation _defaultsceneroot))
  (bind (_x _y _z) (Math|Vector|BreakVector _returnvalue))
  ;[0.1912 0.4072 0.1248] Comment
  (Variables|Default|GetCurrentFocusObject
    (:then)
    (:else
      (bind _returnvalue_2 (Game|SpawnActorfromClass (Variables|Default|GetClass%20Filter) (Math|Transform|MakeTransform (Math|Vector|MakeVector _x _y (+ _z 1e+01)) "0, 0, 0" "1.000000,1.000000,1.000000") "Undefined" "MultiplyWithRoot" 0 0))
      (Variables|Default|SetCurrentFocusObject _returnvalue_2))))

(fn ConstructionScript)
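; Actor for the current potion, which shows its liquid and snaps in and out of view.
; On BeginPlay it caches positions from two reference actors, sets a default water material and starts at the off-screen spot.
; Events teleport the root between those spots without interpolation, or apply the material stored in PotionComponent's potion data to the water mesh.
; ClearPotion resets that data to the unknown potion but does not refresh the material itself.
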(event Custom|ApplyMaterials
  (Rendering|Material|SetMaterial (Variables|Default|GetPotion%20Water) 0 (.MaterialsPotion (Utilities|Struct|BreakS_PotionRecipe (Variables|/Game/_PotionCraft/BP/BP_Potion/PotionComponent.PotionComponent_C|GetThis%20Potion (Variables|Default|GetPotionComponent))))))

(event Custom|ClearPotion
  (Variables|/Game/_PotionCraft/BP/BP_Potion/PotionComponent.PotionComponent_C|SetThis%20Potion (Variables|Default|GetPotionComponent) (Utilities|Struct|MakeS_PotionRecipe "Unknow" "()" "()" "NewEnumerator2" "/Game/_PotionCraft/Materials/PotionMat/Mat_Unknow.Mat_Unknow")))

(event Custom|GetPotionInScreen
  (Transformation|SetWorldTransform (Variables|Default|GetDefaultSceneRoot) (stale EventBeginPlay _output_get_2) false false))

(event Custom|GetPotionOutScreen
  (Transformation|SetWorldTransform (Variables|Default|GetDefaultSceneRoot) (stale EventBeginPlay _output_get) false false))

(event EventBeginPlay
  (Rendering|Material|SetMaterial (Variables|Default|GetPotion%20Water) 0 "/Engine/BufferVisualization/Anisotropy.Anisotropy")
  (bind _output_get (Variables|Default|SetOut%20Screen%20Transform (Math|Transform|MakeTransform (Transformation|GetActorLocation (Variables|Default|GetOut%20Screen%20Ref)) "0, 0, 0" "1.000000,1.000000,1.000000")))
  (bind _output_get_2 (Variables|Default|SetIn%20Screen%20Transform (Math|Transform|MakeTransform (Transformation|GetActorLocation (Variables|Default|GetIn%20Screen%20Ref)) "0, 0, 0" "1.000000,1.000000,1.000000")))
  (Transformation|SetWorldTransform (Variables|Default|GetDefaultSceneRoot) _output_get false false))

(fn ConstructionScript)
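; BP_PotionRandom is a potion Blueprint that picks a random recipe from the DTPotionInfo data table.
; BeginPlay and the RandomeNewPotion event share one roll, which stores a random row in PotionComponent.ThisPotion.
; DebugCocktail then prints that recipe's name, herb and crystal keys, liquid and material for debugging.
; A separate AddHerb function, not called here, tallies ingredient counts in the PotionRecipesHerb map.
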(event Custom|RandomeNewPotion
  ;[1 1 1] Get Random Potion
  (bind _outrownames (DataTable|GetDataTableRowNames (Variables|Potion|GetDT_PotionInfo)))
  (bind _returnvalue (Utilities|GetDataTableRow (Variables|Potion|GetDT_PotionInfo) (.OutItem (Utilities|Array|Random _outrownames)))
    (:then
      (bind _output_get (Variables|/Game/_PotionCraft/BP/BP_Potion/PotionComponent.PotionComponent_C|SetThis%20Potion (Variables|Default|GetPotionComponent) _returnvalue))
      (CallFunction|DebugCocktail _output_get))
    (:RowNotFound
      (Development|PrintString "The fuck is this" true true "(R=0.000000,G=0.660000,B=1.000000,A=1.000000)" 1e+01))))

(event EventBeginPlay
  (Utilities|FlowControl|Sequence
    (:then_0
      ;[1 1 1] Get Random Potion
      (bind _outrownames (DataTable|GetDataTableRowNames (Variables|Potion|GetDT_PotionInfo)))
      (bind _returnvalue (Utilities|GetDataTableRow (Variables|Potion|GetDT_PotionInfo) (.OutItem (Utilities|Array|Random _outrownames)))
        (:then
          (bind _output_get (Variables|/Game/_PotionCraft/BP/BP_Potion/PotionComponent.PotionComponent_C|SetThis%20Potion (Variables|Default|GetPotionComponent) _returnvalue))
          (CallFunction|DebugCocktail _output_get))
        (:RowNotFound
          (Development|PrintString "The fuck is this" true true "(R=0.000000,G=0.660000,B=1.000000,A=1.000000)" 1e+01))))))

(fn ConstructionScript)

(fn DebugCocktail
  (params (S_PotionRecipe :type S%20Potion%20Recipe%20Structure%20%28by%20ref%29))
  (bind (_potionname _herb _crystal _liquid _materialspotion) (Utilities|Struct|BreakS_PotionRecipe S_PotionRecipe))
  (Development|PrintString _potionname true true "(R=0.000000,G=0.660000,B=1.000000,A=1.000000)" 1e+01)
  (if (Utilities|Map|IsNotEmpty _herb)
    (bind _keys (Utilities|Map|Keys _herb))
    (bind _array_element (Utilities|Array|ForEachLoopwithBreak _keys)
      (:LoopBody
        (Development|PrintString (Utilities|String|EnumtoString _array_element) true true "(R=0.719183,G=0.000000,B=1.000000,A=1.000000)" 1e+01))
      (:Completed
        (if (Utilities|Map|IsNotEmpty _crystal) :!label _label
          (Utilities|Map|Keys _crystal)
          (bind _array_element_2 (Utilities|Array|ForEachLoopwithBreak "NewEnumerator8")
            (:LoopBody
              (Development|PrintString (Utilities|String|EnumtoString _array_element_2) true true "(R=1.000000,G=0.000000,B=0.647163,A=1.000000)" 1e+01))
            (:Completed
              (Development|PrintString (Utilities|String|EnumtoString _liquid) true true "(R=0.277329,G=0.000000,B=1.000000,A=1.000000)" 1e+01 :!label _label_2)
              (Development|PrintString (Utilities|GetDisplayName _materialspotion))))
          (else
            (goto _label_2)))))
    (else
      (goto _label))))

(fn AddHerb
  (params (KeyHerbORLiquid :type Enum_Herbs%20Enum%20%28by%20ref%29 :default "NewEnumerator8"))
  (bind _potion_recipes_herb (Variables|Potion|GetPotion%20Recipes%20Herb))
  (bind (_value _returnvalue) (Utilities|Map|Find _potion_recipes_herb KeyHerbORLiquid))
  (if _returnvalue
    (Utilities|Map|Add _potion_recipes_herb KeyHerbORLiquid (+ _value 1))
    (else
      (Utilities|Map|Add _potion_recipes_herb KeyHerbORLiquid 1))))
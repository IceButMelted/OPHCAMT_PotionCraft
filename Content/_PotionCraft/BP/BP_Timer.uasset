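; BP_Timer is a countdown timer actor that tracks minutes and seconds until time runs out.
; Tick feeds a one-second Delay, whose latent retrigger blocking paces the countdown to roughly one step per second.
; Each step decrements Second, borrowing from Minute at zero, and prints the remaining time as a debug string.
; When both reach zero it sets TimeUps, which stops further counting.
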(event Collision|EventActorBeginOverlap
  (params (OtherActor :type Actor%20Object%20Reference)))

(event EventTick
  (params (DeltaSeconds :type Float%20%28single-precision%29))
  (Utilities|FlowControl|Delay 1.0)
  (if (not (Variables|Default|GetTimeUps))
    (if (== (Variables|Default|GetSecond) 0)
      (if (== (Variables|Default|GetMinute) 0)
        (Variables|Default|SetTimeUps true)
        (else
          (Variables|Default|SetMinute (- (Variables|Default|GetMinute) 1))
          (Variables|Default|SetSecond 59)
          (Development|PrintString (Utilities|String|ToString(Text) (Utilities|Text|FormatText "{a};{b}" (Variables|Default|GetMinute) (Variables|Default|GetSecond))) :!label _label)))
      (else
        (Variables|Default|SetSecond (- (Variables|Default|GetSecond) 1))
        (goto _label)))))

(fn ConstructionScript)